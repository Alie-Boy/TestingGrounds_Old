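; AI controller for guard NPCs that runs a guard behavior tree and tracks the player as an enemy.
; On BeginPlay it sets up the PatrolData blackboard and starts the GuradBehaviour tree.
; AI Perception updates feed a helper that sets the Enemy blackboard key when a Player-tagged actor is sensed and clears it when that stimulus is lost.
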(event `self.ReceiveBeginPlay`
  (bind _blackboardcomponent (`self.UseBlackboard` "/Game/Character/AI/PatrolData.PatrolData"))
  (`self.RunBehaviorTree` "/Game/Character/AI/GuradBehaviour.GuradBehaviour")
  (set `self.BlackboardComp` _blackboardcomponent))

(event `self.AIPerception.OnTargetPerceptionUpdated`
  (params (Actor :type "Actor Object Reference") (Stimulus :type "AIStimulus Structure"))
  (`self.Update Blackboard Enemy Key` Stimulus Actor))

(fn `Update Blackboard Enemy Key`
  (params (AIStimulus :type "AIStimulus Structure (by ref)") (Actor :type "Actor Object Reference"))
  (bind _blackboardcomp (`self.BlackboardComp`))
  (if (`self.ActorHasTag` Actor "Player")
    (if (`.bSuccessfullySensed` (break `AIStimulus` AIStimulus))
      (`BlackboardComponent.SetValueAsObject` _blackboardcomp "Enemy" Actor)
      (else
        (`BlackboardComponent.ClearValue` _blackboardcomp "Enemy")))))

(fn `UserConstructionScript`)