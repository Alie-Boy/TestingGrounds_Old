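; BP_Tile is a level tile for infinite terrain that scatters containers, rocks, boxes, cover and AI pawns on BeginPlay.
; Its door starts locked, opens when the player enters LockingVolume, then relocks on exit while the game mode spawns another tile and records a conquest.
; GCVolume overlap by the player destroys the tile and its attached actors.
; GetAttachTransform exposes the Arrow's world transform as an attach point.
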(event `self.ReceiveBeginPlay`
  (`self.Lock`)
  (`self.PlaceActors` "/Game/Levels/Props/BP_Container.BP_Container_C" 1 3)
  (`self.PlaceActors` "/Game/Levels/Props/BP_Rock01_High.BP_Rock01_High_C" 2 3 250)
  (`self.PlaceActors` "/Game/Levels/Props/BP_Rock05_High.BP_Rock05_High_C" 3 4 300)
  (`self.PlaceActors` "/Game/Levels/Props/BP_Rock17_High.BP_Rock17_High_C" 1 2 250)
  (`self.PlaceActors` "/Game/Levels/Props/BP_Box.BP_Box_C" 4 6 100)
  (`self.PlaceActors` "/Game/Levels/Props/BP_SandbagCover.BP_SandbagCover_C" 1 3 250 2.0 3.0)
  (`self.PlaceAIPawns` "/Game/Character/Behaviour/BP_Character.BP_Character_C" 2 4 100))

(event `self.LockingVolume.OnComponentBeginOverlap`
  (params (OverlappedComponent :type "PrimitiveComponent Object Reference") (OtherActor :type "Actor Object Reference") (OtherComp :type "PrimitiveComponent Object Reference") (OtherBodyIndex :type Integer) (bFromSweep :type Boolean) (SweepResult :type "HitResult Structure (by ref)"))
  (`self.Is Player Actor` OtherActor)
  (`self.Unlock`))

(event `self.LockingVolume.OnComponentEndOverlap`
  (params (OverlappedComponent :type "PrimitiveComponent Object Reference") (OtherActor :type "Actor Object Reference") (OtherComp :type "PrimitiveComponent Object Reference") (OtherBodyIndex :type Integer))
  (bind _asbp_infinite_terrain_game_mode (cast `/Game/BP_InfiniteTerrainGameMode` (`GameplayStatics.GetGameMode`) :!pure true))
  (`self.Is Player Actor` OtherActor)
  (`self.Lock`)
  (`/Game/BP_InfiniteTerrainGameMode.Spawn Tile` _asbp_infinite_terrain_game_mode)
  (`InfiniteTerrainGameMode.NewTileConquered` _asbp_infinite_terrain_game_mode))

(event `self.GCVolume.OnComponentBeginOverlap`
  (params (OverlappedComponent :type "PrimitiveComponent Object Reference") (OtherActor :type "Actor Object Reference") (OtherComp :type "PrimitiveComponent Object Reference") (OtherBodyIndex :type Integer) (bFromSweep :type Boolean) (SweepResult :type "HitResult Structure (by ref)"))
  (`self.Is Player Actor` OtherActor)
  (bind _children (`/DatasmithContent/Blueprints/FBXImporter/FBXImporterUtils.GetAllAttachedActors` self))
  (for _array_element _children
    (`self.K2_DestroyActor` _array_element))
  (`self.K2_DestroyActor`))

(fn `Get Attach Transform`
  (returns (AttachTransform :type "Transform Structure"))
  (return (`SceneComponent.K2_GetComponentToWorld` (`self.Arrow`))))

(fn `Lock`
  (bind _door (`self.Door`))
  (`PrimitiveComponent.SetCollisionEnabled` _door "QueryAndPhysics")
  (`PrimitiveComponent.SetMaterial` _door 0 "/Game/Geometry/Meshes/MI_Barrier_Red.MI_Barrier_Red"))

(fn `Unlock`
  (bind _door (`self.Door`))
  (`PrimitiveComponent.SetCollisionEnabled` _door "NoCollision")
  (`PrimitiveComponent.SetMaterial` _door 0 "/Game/Geometry/Meshes/MI_Barrier_Green.MI_Barrier_Green"))

(fn `UserConstructionScript`)