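; Behavior tree task that picks the next patrol waypoint for an AI-controlled ThirdPersonCharacter.
; It reads the pawn's PatrolPoints array, writes the entry at the blackboard Index to the Waypoint key, then increments Index and finishes successfully.
; Index resets to zero only after equalling the array length, so one pass per cycle reads past the last point.
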(event `self.ReceiveExecuteAI`
  (params (OwnerController :type "AIController Object Reference") (ControlledPawn :type "Pawn Object Reference"))
  (`self.Get Patrol Points` ControlledPawn)
  (`self.Set Next Waypoint`)
  (`self.Cycle Index`)
  (`self.FinishExecute` true))

(fn `Cycle Index`
  (bind _index (`self.Index`))
  (bind _returnvalue (`BTFunctionLibrary.GetBlackboardValueAsInt` _index))
  (if (== _returnvalue (`KismetArrayLibrary.Array_Length` (`self.Patrol Points`)))
    (`BTFunctionLibrary.SetBlackboardValueAsInt` _index)
    (else
      (`BTFunctionLibrary.SetBlackboardValueAsInt` _index (+ _returnvalue 1)))))

(fn `Get Patrol Points`
  (params (Object :type "Object Object Reference"))
  (bind _asthird_person_character (cast `/Game/Trash/ThirdPersonCharacter` Object))
  (set `self.Patrol Points` (`/Game/Trash/ThirdPersonCharacter.Patrol Points` _asthird_person_character)))

(fn `Set Next Waypoint`
  (`BTFunctionLibrary.SetBlackboardValueAsObject` (`self.Waypoint`) (`|GetArrayItem` (`self.Patrol Points`) (`BTFunctionLibrary.GetBlackboardValueAsInt` (`self.Index`)))))